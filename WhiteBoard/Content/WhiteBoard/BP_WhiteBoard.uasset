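; Interactive whiteboard actor that the player draws on with red, black or blue pens.
; F toggles a blended camera view of the board and the cursor, while number keys switch pen colour and briefly show as hints at start.
; Each tick a mouse-ray trace positions the pen while the board is in use.
; Holding left mouse spawns ink decals at the hit, even outside board view, and plays a pen-press timeline.
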(event EventTick
  (params (DeltaSeconds :type Float%20%28single-precision%29))
  (bind _returnvalue (Game|GetPlayerController 0))
  (bind _mainpen (Variables|Default|GetMainPen))
  (bind (_worldlocation _worlddirection) (Game|Player|ConvertMouseLocationToWorldSpace _returnvalue))
  ;[1 1 1] Event Tick
  (Utilities|FlowControl|Sequence
    (:then_0
      ;[1 1 1] Line Trace From Mouse Pointer
      (bind _outhit (Collision|LineTraceByChannel _worldlocation (+ _worldlocation (* _worlddirection 1e+03)) "TraceTypeQuery2" false 0 "None"))
      ;[1 1 1] Spawn Decal And Animate Pen Pressing
      (if (Variables|Default|Getlmbheld)
        (Rendering|Decal|SpawnDecalatLocation (Variables|Default|GetPenColour) "2.000000,2.000000,2.000000" (.Location (Collision|BreakHitResult _outhit)) "0.000000,90.000000,90.000000" 0.0)
        (bind _newtrack_0 (Timeline|PushPenToBoard Play)
          (:Update
            (Transformation|SetRelativeLocation _mainpen (+ _newtrack_0 (Variables|/Script/Engine.SceneComponent|GetRelativeLocation _mainpen)) false)))
        (else
          (Timeline|PushPenToBoard Reverse))))
    (:then_1
      ;[1 1 1] Update Pen Location To Mouse Pointer
      (if (Variables|Default|GetUsingWhiteBoard)
        (Transformation|SetWorldLocation (Variables|Default|GetMainPen) (+ "0.000000,30.000000,0.000000" (.Location (Collision|BreakHitResult _outhit))) false)))))

(event EventBeginPlay
  (bind _3 (Variables|Default|Get3))
  ;[1 1 1] Begin Play Enable Input
  (Input|EnableInput (Game|GetPlayerController 0))
  ;;[1 1 1] Display and hide the information numbers that display how to change pens
  (Rendering|SetVisibility _3 true false)
  (Utilities|FlowControl|Delay 3.0)
  (Rendering|SetVisibility _3 false false))

(event Input|KeyboardEvents|1
  (:Pressed
    (Rendering|Material|SetMaterial (Variables|Default|GetMainPen) 0 "/Game/WhiteBoard/WhiteBoardPen/WhiteBoardPen_Red_Mat.WhiteBoardPen_Red_Mat")
    (Rendering|SetVisibility (Variables|Default|GetRedPen) false false)
    (Rendering|SetVisibility (Variables|Default|GetBluePen) true false)
    (Variables|Default|SetPenColour "/Game/WhiteBoard/Materials/Pen_Red.Pen_Red")))

(event Input|MouseEvents|LeftMouseButton
  ;[1 1 1] Set Left Mouse button Held Variable
  (:Pressed
    (Variables|Default|Setlmbheld true))
  (:Released
    (Variables|Default|Setlmbheld false)))

(event Input|KeyboardEvents|2
  (:Pressed
    (Rendering|Material|SetMaterial (Variables|Default|GetMainPen) 0 "/Game/WhiteBoard/WhiteBoardPen/WhiteBoardPen_Black_Mat.WhiteBoardPen_Black_Mat")
    (Rendering|SetVisibility (Variables|Default|GetBlackPen) false false)
    (Rendering|SetVisibility (Variables|Default|GetBluePen) true false)
    (Variables|Default|SetPenColour "/Game/WhiteBoard/Materials/Pen_Black.Pen_Black")))

(event Input|KeyboardEvents|3
  (:Pressed
    (Rendering|Material|SetMaterial (Variables|Default|GetMainPen) 0 "/Game/WhiteBoard/WhiteBoardPen/WhiteBoardPen_BLue_Mat.WhiteBoardPen_BLue_Mat")
    (Rendering|SetVisibility (Variables|Default|GetBluePen) false false)
    (Rendering|SetVisibility (Variables|Default|GetBlackPen) true false)
    (Variables|Default|SetPenColour "/Game/WhiteBoard/Materials/Pen_Blue.Pen_Blue")))

(event Input|KeyboardEvents|F
  (bind _returnvalue (Game|GetPlayerController 0))
  ;[1 1 1] Change Camera To WhiteBoard
  (:Pressed
    (Utilities|FlowControl|FlipFlop
      (:A
        (Game|Player|SetViewTargetwithBlend _returnvalue self 1.0 "VTBlend_Linear" 0.0 false)
        (Variables|/Script/Engine.PlayerController|SetbShowMouseCursor _returnvalue true)
        (Variables|Default|SetUsingWhiteBoard true))
      (:B
        (Game|Player|SetViewTargetwithBlend _returnvalue (Game|Player|GetPlayerPawn 0) 1.0 "VTBlend_Linear" 0.0 false)
        (Variables|/Script/Engine.PlayerController|SetbShowMouseCursor _returnvalue false)
        (Variables|Default|SetUsingWhiteBoard false)))))

(fn ConstructionScript
  (Rendering|Material|SetMaterial (Variables|Default|GetBluePen) 0 "/Game/WhiteBoard/WhiteBoardPen/WhiteBoardPen_BLue_Mat.WhiteBoardPen_BLue_Mat")
  (Rendering|Material|SetMaterial (Variables|Default|GetRedPen) 0 "/Game/WhiteBoard/WhiteBoardPen/WhiteBoardPen_Red_Mat.WhiteBoardPen_Red_Mat")
  (Rendering|Material|SetMaterial (Variables|Default|GetBlackPen) 0 "/Game/WhiteBoard/WhiteBoardPen/WhiteBoardPen_Black_Mat.WhiteBoardPen_Black_Mat"))